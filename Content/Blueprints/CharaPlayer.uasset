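; Player character for a 2D side-scrolling platformer, built on Paper2D flipbook sprites.
; On BeginPlay it adds the Platforming Enhanced Input context, whose actions drive jumping and movement along X, flipping control yaw to face the travel direction.
; Tick picks the run, idle, jump or fall flipbook from ground state and velocity.
; DashForward and DashReset hold disabled logic for a timeline-driven, swept dash with attack and dodge resets.
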(event Custom|DashForward
  (Utilities|FlowControl|DoOnce false
    (:Completed
      (bind _новая_дорожка_0 (Timeline|Timeline PlayFromStart)
        (:Update
          (Transformation|AddActorWorldOffset (Math|Vector|MakeVector (* _новая_дорожка_0 (select (Variables|Default|GetJump%20Right?) -2e+03 2e+03) (select (Variables|Default|GetFocused) 0.9 2.0) (Utilities|Time|GetWorldDeltaSeconds)) 0.0 0.0) true))))))

(event Custom|DashReset
  (Utilities|FlowControl|Sequence
    (:then_0
      (Utilities|FlowControl|DoOnce false) ; enters at Reset
    )
    (:then_1
      (Utilities|FlowControl|DoOnce false ; enters at Reset
        (:Completed
          (CallFunction|ResetAttackCounter)
          (bind (_jumpright_ _focused_) (CallFunction|WheretoDodge))
          (Variables|Default|SetFocused _focused_)
          (Variables|Default|SetJump%20Right? _jumpright_))))))

(event Input|EnhancedActionEvents|EnhancedInputActionJump
  (params (ActionValue :type Boolean) (ElapsedSeconds :type Float%20%28double-precision%29) (TriggeredSeconds :type Float%20%28double-precision%29) (InputAction :type Input%20Action%20Object%20Reference :default "/Game/Input/Actions/Jump.Jump"))
  ;[0.15 0.15 0.15 0.5] Механика прыжка
  (:Started
    (Character|Jump))
  (:Completed
    (Character|StopJumping)))

(event Input|EnhancedActionEvents|EnhancedInputActionMove
  (params (ActionValue :type Float%20%28double-precision%29) (ElapsedSeconds :type Float%20%28double-precision%29) (TriggeredSeconds :type Float%20%28double-precision%29) (InputAction :type Input%20Action%20Object%20Reference :default "/Game/Input/Actions/Move.Move"))
  ;[0.15 0.15 0.15 0.5] Разворот спрайта на 180 при развороте
  (Pawn|Input|AddMovementInput "1.000000,0.000000,0.000000" ActionValue false)
  (Pawn|SetControlRotation (Pawn|GetController) (select (> ActionValue 0.0) (Math|Rotator|MakeRotator 0.0 0.0 0.0) (Math|Rotator|MakeRotator 0.0 0.0 1.8e+02))))

(event EventBeginPlay
  ;[0.15 0.15 0.15 0.5] Назначение клавиш управления
  (bind _asplayer_controller (Utilities|Casting|CastToPlayerController (Pawn|GetController)))
  (Input|AddMappingContext (PlayerController|LocalPlayerSubsystems|GetEnhancedInputLocalPlayerSubsystem _asplayer_controller) "/Game/Input/Platforming.Platforming" 0 "(bIgnoreAllPressedKeysUntilRelease=True,bForceImmediately=False,bNotifyUserSettings=False)"))

(event EventTick
  (params (DeltaSeconds :type Float%20%28single-precision%29))
  ;[0.15 0.15 0.15 0.5] Замена спрайтов в зависимости от состояния игрока
  (if (AI|Components|NavMovement|IsMovingonGround (Variables|Character|GetCharacterMovement))
    (if (> (Math|Vector|VectorLength (Transformation|GetVelocity)) 0.0)
      (Sprite|SetFlipbook (Variables|Default|GetSprite) "/Game/PaperAssets/Adventurer/Textbooks/adventurer_run.adventurer_run")
      (else
        (Sprite|SetFlipbook (Variables|Default|GetSprite) "/Game/PaperAssets/Adventurer/Textbooks/adventurer_idle.adventurer_idle")))
    (elif (< (.z (Transformation|GetVelocity)) -1e+02)
      (Sprite|SetFlipbook (Variables|Default|GetSprite) "/Game/PaperAssets/Adventurer/Textbooks/adventurer_fall.adventurer_fall")
      (else
        (Sprite|SetFlipbook (Variables|Default|GetSprite) "/Game/PaperAssets/Adventurer/Textbooks/adventurer_jump.adventurer_jump")))))

(fn ConstructionScript)